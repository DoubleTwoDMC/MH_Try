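; Player character for an ALS-style shooter with Enhanced Input movement, aiming, crouching, jumping and unarmed, pistol or rifle loadouts.
; Weapon switching relinks anim class layers and moves gun meshes between sockets, while SetMoveState applies movement settings from DT_MoveSetting per stance and weapon.
; State, weapon and traced ground height go to the AnimInstance via messages.
; Fire and reload play paired character and weapon animations, with timer-gated fire rate.
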(event Custom|RifleFireOver
  (Variables|Default|SetCanFire true))

(event Custom|PistolFireOver
  (Variables|Default|SetCanFire true))

(event Input|EnhancedActionEvents|EnhancedInputActionIA_SwitchWeapon
  (params (ActionValue :type Float%20%28double-precision%29) (ElapsedSeconds :type Float%20%28double-precision%29) (TriggeredSeconds :type Float%20%28double-precision%29) (InputAction :type Input%20Action%20Object%20Reference :default "/Game/ALS/Input/InputActions/IA_SwitchWeapon.IA_SwitchWeapon"))
  (bind _mesh (Variables|Character|GetMesh))
  (switch int (Math|Float|Truncate ActionValue)
    (:1
      (if (Utilities|Enum|NotEqual(Enum) (Variables|Default|GetEquitGun) "NewEnumerator0")
        (Variables|Default|SetEquitGun "NewEnumerator0")
        (Components|SkeletalMesh|AnimationBlueprintLinking|LinkAnimClassLayers _mesh "/Game/ALS/AnimationBluePrint/ABP_Layers_UnArmed.ABP_Layers_UnArmed_C")
        (Transformation|AttachComponentToComponent (Variables|Default|GetPistol) (Variables|Character|GetMesh) (.PistolUnequipment (Utilities|Struct|BreakS_WeaponSocket (Variables|Default|GetWeaponSocket))) "KeepRelative" "KeepRelative" "KeepRelative" true)
        (Transformation|AttachComponentToComponent (Variables|Default|GetRifle) (Variables|Character|GetMesh) (.RifleUnequipment (Utilities|Struct|BreakS_WeaponSocket (Variables|Default|GetWeaponSocket))) "KeepRelative" "KeepRelative" "KeepRelative" true)
        (CallFunction|SetMoveState (Variables|Default|GetMoveState) :!label _label)
        (Class|BPIAnimationInterface|ReciveEquiptGum(Message) (Components|SkeletalMesh|GetAnimInstance (Variables|Character|GetMesh)) (Variables|Default|GetEquitGun))))
    (:2
      (if (Utilities|Enum|NotEqual(Enum) (Variables|Default|GetEquitGun) "NewEnumerator1")
        (Variables|Default|SetEquitGun "NewEnumerator1")
        (Variables|Default|SetCanFire true)
        (Components|SkeletalMesh|AnimationBlueprintLinking|LinkAnimClassLayers _mesh "/Game/ALS/AnimationBluePrint/ABP_Layers_Pistol.ABP_Layers_Pistol_C")
        (Transformation|AttachComponentToComponent (Variables|Default|GetPistol) (Variables|Character|GetMesh) (.WeaponEquipment (Utilities|Struct|BreakS_WeaponSocket (Variables|Default|GetWeaponSocket))) "KeepRelative" "KeepRelative" "KeepRelative" true)
        (Transformation|AttachComponentToComponent (Variables|Default|GetRifle) (Variables|Character|GetMesh) (.RifleUnequipment (Utilities|Struct|BreakS_WeaponSocket (Variables|Default|GetWeaponSocket))) "KeepRelative" "KeepRelative" "KeepRelative" true)
        (goto _label)))
    (:3
      (if (Utilities|Enum|NotEqual(Enum) (Variables|Default|GetEquitGun) "NewEnumerator2")
        (Variables|Default|SetEquitGun "NewEnumerator2")
        (Variables|Default|SetCanFire true)
        (Components|SkeletalMesh|AnimationBlueprintLinking|LinkAnimClassLayers _mesh "/Game/ALS/AnimationBluePrint/ABP_Layers_Rifle.ABP_Layers_Rifle_C")
        (Transformation|AttachComponentToComponent (Variables|Default|GetRifle) (Variables|Character|GetMesh) (.WeaponEquipment (Utilities|Struct|BreakS_WeaponSocket (Variables|Default|GetWeaponSocket))) "KeepRelative" "KeepRelative" "KeepRelative" true)
        (Transformation|AttachComponentToComponent (Variables|Default|GetPistol) (Variables|Character|GetMesh) (.PistolUnequipment (Utilities|Struct|BreakS_WeaponSocket (Variables|Default|GetWeaponSocket))) "KeepRelative" "KeepRelative" "KeepRelative" true)
        (goto _label)))))

(event Input|EnhancedActionEvents|EnhancedInputActionIA_Look
  (params (ActionValue :type Vector%202D%20Structure) (ElapsedSeconds :type Float%20%28double-precision%29) (TriggeredSeconds :type Float%20%28double-precision%29) (InputAction :type Input%20Action%20Object%20Reference :default "/Game/ALS/Input/InputActions/IA_Look.IA_Look"))
  (bind (_x _y) (Math|Vector2D|BreakVector2D ActionValue))
  (Pawn|Input|AddControllerYawInput _x)
  (Pawn|Input|AddControllerPitchInput _y))

(event Input|EnhancedActionEvents|EnhancedInputActionIA_Move
  (params (ActionValue :type Vector%202D%20Structure) (ElapsedSeconds :type Float%20%28double-precision%29) (TriggeredSeconds :type Float%20%28double-precision%29) (InputAction :type Input%20Action%20Object%20Reference :default "/Game/ALS/Input/InputActions/IA_Move.IA_Move"))
  (bind (_x _y) (Math|Vector2D|BreakVector2D ActionValue))
  (bind _returnvalue (Pawn|GetControlRotation :!class /Script/Engine.Pawn))
  (Pawn|Input|AddMovementInput (Math|Rotator|GetRotationXVector (Math|Rotator|MakeRotator 0.0 0.0 (.yaw (Pawn|GetControlRotation :!class /Script/Engine.Pawn)))) _y false)
  (Pawn|Input|AddMovementInput (Math|Vector|GetRightVector (Math|Rotator|MakeRotator (.roll _returnvalue) 0.0 (.yaw _returnvalue))) _x false))

(event Input|EnhancedActionEvents|EnhancedInputActionIA_Jump
  (params (ActionValue :type Boolean) (ElapsedSeconds :type Float%20%28double-precision%29) (TriggeredSeconds :type Float%20%28double-precision%29) (InputAction :type Input%20Action%20Object%20Reference :default "/Game/ALS/Input/InputActions/IA_Jump.IA_Jump"))
  (:Started
    (Character|Jump))
  (:Completed
    (Character|StopJumping)))

(event Input|EnhancedActionEvents|EnhancedInputActionIA_Aim
  (params (ActionValue :type Boolean) (ElapsedSeconds :type Float%20%28double-precision%29) (TriggeredSeconds :type Float%20%28double-precision%29) (InputAction :type Input%20Action%20Object%20Reference :default "/Game/ALS/Input/InputActions/IA_Aim.IA_Aim"))
  (bind _movestate (Variables|Default|GetMoveState))
  (:Started
    (switch Utilities|FlowControl|Switch|SwitchonEMoveState _movestate
      (:NewEnumerator0
        (CallFunction|SetMoveState "NewEnumerator1" :!label _label)
        (Variables|Default|SetCanFire true)
        (bind _springarmline (Timeline|AimSpringArmChange Play)
          (:Update
            (Variables|/Script/Engine.SpringArmComponent|SetTargetArmLength (Variables|Default|GetSpringArm) (Math|Float|Lerp 3.5e+02 1.5e+02 _springarmline)))))
      (:NewEnumerator1
        (goto _label))
      (:NewEnumerator2
        (CallFunction|SetMoveState "NewEnumerator2")
        (Variables|Default|SetCanFire true)
        (Timeline|AimSpringArmChange Play))))
  (:Completed
    (switch Utilities|FlowControl|Switch|SwitchonEMoveState _movestate
      (:NewEnumerator0
        (CallFunction|SetMoveState "NewEnumerator0" :!label _label_2)
        (Variables|Default|SetCanFire false)
        (Timeline|AimSpringArmChange Reverse))
      (:NewEnumerator1
        (goto _label_2))
      (:NewEnumerator2
        (CallFunction|SetMoveState "NewEnumerator2")
        (Variables|Default|SetCanFire true)
        (Timeline|AimSpringArmChange Reverse)))))

(event Input|EnhancedActionEvents|EnhancedInputActionIA_Crouch
  (params (ActionValue :type Boolean) (ElapsedSeconds :type Float%20%28double-precision%29) (TriggeredSeconds :type Float%20%28double-precision%29) (InputAction :type Input%20Action%20Object%20Reference :default "/Game/ALS/Input/InputActions/IA_Crouch.IA_Crouch"))
  (:Started
    (switch Utilities|FlowControl|Switch|SwitchonEMoveState (Variables|Default|GetMoveState)
      (:NewEnumerator0
        (CallFunction|SetMoveState "NewEnumerator2" :!label _label)
        (Character|Crouch))
      (:NewEnumerator1
        (goto _label))
      (:NewEnumerator2
        (CallFunction|SetMoveState "NewEnumerator0")
        (Character|UnCrouch)))))

(event Input|EnhancedActionEvents|EnhancedInputActionIA_Fire
  (params (ActionValue :type Boolean) (ElapsedSeconds :type Float%20%28double-precision%29) (TriggeredSeconds :type Float%20%28double-precision%29) (InputAction :type Input%20Action%20Object%20Reference :default "/Game/ALS/Input/InputActions/IA_Fire.IA_Fire"))
  (switch Utilities|FlowControl|Switch|SwitchonEMoveState (Variables|Default|GetMoveState)
    (:NewEnumerator0
      (if (Math|Float|NearlyEqual(Float) (Math|Vector|VectorLength (Variables|/Script/Engine.MovementComponent|GetVelocity (Variables|Character|GetCharacterMovement))) 0.0 1e-06)
        (if (Variables|Default|GetCanFire) :!label _label
          (Variables|Default|SetCanFire false)
          (switch Utilities|FlowControl|Switch|SwitchonEGun (Variables|Default|GetEquitGun)
            (:NewEnumerator0
              (Variables|Default|SetCanFire false))
            (:NewEnumerator1
              (Utilities|Time|SetTimerbyEvent (delegate Custom|PistolFireOver) 0.5)
              (Animation|Montage|PlayMontage (Variables|Character|GetMesh) "/Game/ALS/Animation/Pistol/Gun/AM_Pistol_Fire_Montage.AM_Pistol_Fire_Montage"
                (:then
                  (Components|Animation|PlayAnimation (Variables|Default|GetPistol) "/Game/ALS/Animation/Pistol/Gun/Weap_Pistol_Fire.Weap_Pistol_Fire" false)
                  (Audio|PlaySoundatLocation "/Game/ALS/MetaSounds/MS_Fire_Pistol.MS_Fire_Pistol" (.Location (Math|Transform|BreakTransform (Transformation|GetBoneTransform (Variables|Default|GetPistol) "Barrel" "RTS_World"))) "0, 0, 0" 1.0 1.0 0.0 0 0 0 0))))
            (:NewEnumerator2
              (Utilities|Time|SetTimerbyEvent (delegate Custom|RifleFireOver) 0.2)
              (Animation|Montage|PlayMontage (Variables|Character|GetMesh) "/Game/ALS/Animation/Rifle/Gun/AM_Rifle_Fire_Montage.AM_Rifle_Fire_Montage"
                (:then
                  (Components|Animation|PlayAnimation (Variables|Default|GetRifle) "/Game/ALS/Animation/Rifle/Gun/Weap_Rifle_Fire.Weap_Rifle_Fire" false)
                  (Audio|PlaySoundatLocation "/Game/ALS/MetaSounds/MS_Fire_Rifle.MS_Fire_Rifle" (.Location (Math|Transform|BreakTransform (Transformation|GetBoneTransform (Variables|Default|GetRifle) "Barrel" "RTS_World"))) "0, 0, 0" 1.0 1.0 0.0 0 0 0 0))))))))
    (:NewEnumerator1
      (goto _label))
    (:NewEnumerator2
      (goto _label))))

(event Input|EnhancedActionEvents|EnhancedInputActionIA_Reload
  (params (ActionValue :type Boolean) (ElapsedSeconds :type Float%20%28double-precision%29) (TriggeredSeconds :type Float%20%28double-precision%29) (InputAction :type Input%20Action%20Object%20Reference :default "/Game/ALS/Input/InputActions/IA_Reload.IA_Reload"))
  (:Started
    (switch Utilities|FlowControl|Switch|SwitchonEGun (Variables|Default|GetEquitGun)
      (:NewEnumerator1
        (Animation|Montage|PlayMontage (Variables|Character|GetMesh) "/Game/ALS/Animation/Pistol/Gun/AM_Pistol_Reload_Montage.AM_Pistol_Reload_Montage"
          (:then
            (Components|Animation|PlayAnimation (Variables|Default|GetPistol) "/Game/ALS/Animation/Pistol/Gun/Weap_Pistol_Reload.Weap_Pistol_Reload" false))))
      (:NewEnumerator2
        (Animation|Montage|PlayMontage (Variables|Character|GetMesh) "/Game/ALS/Animation/Rifle/Gun/AM_Rifle_Reload_Montage.AM_Rifle_Reload_Montage"
          (:then
            (Components|Animation|PlayAnimation (Variables|Default|GetRifle) "/Game/ALS/Animation/Rifle/Gun/Weap_Rifle_Reload.Weap_Rifle_Reload" false)))))))

(event EventBeginPlay
  (bind _asplayer_controller (Utilities|Casting|CastToPlayerController (Pawn|GetController)))
  (Input|AddMappingContext (PlayerController|LocalPlayerSubsystems|GetEnhancedInputLocalPlayerSubsystem _asplayer_controller) "/Game/ALS/Input/IMC_ALS.IMC_ALS" 0 "(bIgnoreAllPressedKeysUntilRelease=True,bForceImmediately=False,bNotifyUserSettings=False)")
  (Components|SkeletalMesh|AnimationBlueprintLinking|LinkAnimClassLayers (Variables|Character|GetMesh) "/Game/ALS/AnimationBluePrint/ABP_Layers_UnArmed.ABP_Layers_UnArmed_C")
  (CallFunction|SetMoveState "NewEnumerator0")
  (Transformation|AttachComponentToComponent (Variables|Default|GetRifle) (Variables|Character|GetMesh) (.RifleUnequipment (Utilities|Struct|BreakS_WeaponSocket (Variables|Default|GetWeaponSocket))) "KeepRelative" "KeepRelative" "KeepRelative" true)
  (Transformation|AttachComponentToComponent (Variables|Default|GetPistol) (Variables|Character|GetMesh) (.PistolUnequipment (Utilities|Struct|BreakS_WeaponSocket (Variables|Default|GetWeaponSocket))) "KeepRelative" "KeepRelative" "KeepRelative" true))

(event Collision|EventActorBeginOverlap
  (params (OtherActor :type Actor%20Object%20Reference)))

(event EventTick
  (params (DeltaSeconds :type Float%20%28single-precision%29))
  (bind _returnvalue (Transformation|GetActorLocation))
  (bind (_outhit _returnvalue_2) (Collision|SphereTraceByChannel (- _returnvalue (Math|Vector|MakeVector 0.0 0.0 (Variables|/Script/Engine.CapsuleComponent|GetCapsuleHalfHeight (Variables|Collision|GetCapsuleComponent)))) (- _returnvalue "0.000000,0.000000,1000.000000") 5.0 "TraceTypeQuery1" false 0 "None"))
  (if _returnvalue_2
    (bind _output_get (Variables|Default|SetHeight (.Distance (Collision|BreakHitResult _outhit))))
    (Class|BPIAnimationInterface|ReciveJumpHeight(Message) (Components|SkeletalMesh|GetAnimInstance (Variables|Character|GetMesh)) _output_get)))

(event Input|KeyboardEvents|DebugKeySubtract
  (params (Key :type Key%20Structure :default "None") (ActionValue :type Input%20Action%20Value%20Structure))
  (:Pressed
    (Utilities|Time|SetGlobalTimeDilation 0.1)))

(event Input|KeyboardEvents|DebugKeyAdd
  (params (Key :type Key%20Structure :default "None") (ActionValue :type Input%20Action%20Value%20Structure))
  (:Pressed
    (Utilities|Time|SetGlobalTimeDilation 1.0)))

(fn ConstructionScript)

(fn SetMoveState
  (params (MoveState :type EMoveState%20Enum :default "NewEnumerator0"))
  (bind _output_get (Variables|Default|SetMoveState MoveState))
  (Class|BPIAnimationInterface|ReciveMoveState(Message) (Components|SkeletalMesh|GetAnimInstance (Variables|Character|GetMesh)) _output_get)
  (switch Utilities|FlowControl|Switch|SwitchonEMoveState (Variables|Default|GetMoveState)
    (:NewEnumerator0
      (switch Utilities|FlowControl|Switch|SwitchonEGun (Variables|Default|GetEquitGun)
        (:NewEnumerator0
          (bind _returnvalue (Utilities|GetDataTableRow "/Game/ALS/DataTable/DT_MoveSetting.DT_MoveSetting" "UnarmedRun")
            (:then
              (Utilities|SetMoveSettingMacro _returnvalue))))
        (:NewEnumerator1
          (bind _returnvalue_2 (Utilities|GetDataTableRow "/Game/ALS/DataTable/DT_MoveSetting.DT_MoveSetting" "PistolRun")
            (:then
              (Utilities|SetMoveSettingMacro _returnvalue_2))))
        (:NewEnumerator2
          (bind _returnvalue_3 (Utilities|GetDataTableRow "/Game/ALS/DataTable/DT_MoveSetting.DT_MoveSetting" "RifleRun")
            (:then
              (Utilities|SetMoveSettingMacro _returnvalue_3))))))
    (:NewEnumerator1
      (switch Utilities|FlowControl|Switch|SwitchonEGun (Variables|Default|GetEquitGun)
        (:NewEnumerator0
          (bind _returnvalue_4 (Utilities|GetDataTableRow "/Game/ALS/DataTable/DT_MoveSetting.DT_MoveSetting" "UnarmedAimWalk")
            (:then
              (Utilities|SetMoveSettingMacro _returnvalue_4))))
        (:NewEnumerator1
          (bind _returnvalue_5 (Utilities|GetDataTableRow "/Game/ALS/DataTable/DT_MoveSetting.DT_MoveSetting" "PistolAimWalk")
            (:then
              (Utilities|SetMoveSettingMacro _returnvalue_5))))
        (:NewEnumerator2
          (bind _returnvalue_6 (Utilities|GetDataTableRow "/Game/ALS/DataTable/DT_MoveSetting.DT_MoveSetting" "RifleAimWalk")
            (:then
              (Utilities|SetMoveSettingMacro _returnvalue_6))))))
    (:NewEnumerator2
      (switch Utilities|FlowControl|Switch|SwitchonEGun (Variables|Default|GetEquitGun)
        (:NewEnumerator0
          (bind _returnvalue_7 (Utilities|GetDataTableRow "/Game/ALS/DataTable/DT_MoveSetting.DT_MoveSetting" "UnarmedCrouch")
            (:then
              (Variables|/Script/Engine.CharacterMovementComponent|SetMaxWalkSpeedCrouched (Variables|Character|GetCharacterMovement) (.MaxWalkSpeed (Utilities|Struct|BreakS_MoveSetting _returnvalue_7)))
              (Utilities|SetMoveSettingMacro _returnvalue_7))))
        (:NewEnumerator1
          (bind _returnvalue_8 (Utilities|GetDataTableRow "/Game/ALS/DataTable/DT_MoveSetting.DT_MoveSetting" "PistolCrouch")
            (:then
              (Variables|/Script/Engine.CharacterMovementComponent|SetMaxWalkSpeedCrouched (Variables|Character|GetCharacterMovement) (.MaxWalkSpeed (Utilities|Struct|BreakS_MoveSetting _returnvalue_8)))
              (Utilities|SetMoveSettingMacro _returnvalue_8))))
        (:NewEnumerator2
          (bind _returnvalue_9 (Utilities|GetDataTableRow "/Game/ALS/DataTable/DT_MoveSetting.DT_MoveSetting" "RifleCrouch")
            (:then
              (Variables|/Script/Engine.CharacterMovementComponent|SetMaxWalkSpeedCrouched (Variables|Character|GetCharacterMovement) (.MaxWalkSpeed (Utilities|Struct|BreakS_MoveSetting _returnvalue_9)))
              (Utilities|SetMoveSettingMacro _returnvalue_9))))))))